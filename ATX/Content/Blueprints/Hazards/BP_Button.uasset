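; BP_Button is a hazard button that switches connected actors on for a limited time when it takes damage.
; DealDamage sets it active, sends ActivateMessage to every connected actor and sets the button visualizer's material.
; Tick accumulates active time and sends DeactivateMessage once ActiveTime is exceeded.
; The timer is never reset and the material is not changed back on deactivation.
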(event EventDealDamage
  (params (Damage :type Float%20%28single-precision%29) (Source :type Actor%20Object%20Reference))
  ;[1 1 1] Activate On Taking Damage
  (if (not (Variables|Default|GetActive))
    (Variables|Default|SetActive true)
    (for _array_element (Variables|Default|GetConnectedActors)
      (Class|BIBlueprintInteractions|Activate(Message) _array_element)
      (Rendering|Material|SetMaterial (Variables|Default|GetButtonVisualizer) 0 0))))

(event EventTick
  (params (DeltaSeconds :type Float%20%28single-precision%29))
  ;[1 1 1] Deactivate After a while
  (if (Variables|Default|GetActive)
    (bind _output_get (Variables|Default|SetActiverTimer (+ (Variables|Default|GetActiverTimer) DeltaSeconds)))
    (if (> _output_get (Variables|Default|GetActiveTime))
      (Variables|Default|SetActive false)
      (for _array_element (Variables|Default|GetConnectedActors)
        (Class|BIBlueprintInteractions|Deactivate(Message) _array_element)))))

(fn ConstructionScript)