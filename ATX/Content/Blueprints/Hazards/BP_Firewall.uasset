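; BP_Firewall is a hazard actor that damages actors overlapping its DamageCollision while it is active.
; Each Tick sets PlaceholderEffect visibility from the Active flag and, while active, sends DealDamageMessage to overlapping actors, with damage per second scaled by delta time.
; If PeriodicActivation is set, a Tick-accumulated timer waits out a one-time initial delay, then toggles Active using separate activation and deactivation times.
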(event EventTick
  (params (DeltaSeconds :type Float%20%28single-precision%29))
  (if (Variables|Default|GetPeriodicActivation)
    (CallFunction|PeriodicHazardActivation DeltaSeconds))
  (Rendering|SetVisibility (Variables|Default|GetPlaceholderEffect) (Variables|Default|GetActive) false)
  (if (Variables|Default|GetActive)
    (CallFunction|DealHazardDamage DeltaSeconds)))

(fn ConstructionScript)

(fn DealHazardDamage
  (params (DeltaTime :type Float%20%28single-precision%29))
  (for _array_element (Collision|GetOverlappingActors (Variables|Default|GetDamageCollision) 0 :!class /Script/Engine.PrimitiveComponent)
    (Class|BIBlueprintInteractions|DealDamage(Message) _array_element (* DeltaTime (Variables|Default|GetDamagePerSecond)))))

(fn PeriodicHazardActivation
  (params (DeltaTime :type Float%20%28single-precision%29))
  (if (Variables|Default|GetPeriodicDelayUsed)
    (bind _output_get (Variables|Default|SetPeriodicTimer (+ (Variables|Default|GetPeriodicTimer) DeltaTime) :!label _label))
    (if (Variables|Default|GetActive)
      (if (> _output_get (Variables|Default|GetPeriodicDeactivationTime))
        (Variables|Default|SetActive false)
        (Variables|Default|SetPeriodicTimer 0.0 :!label _label_2))
      (elif (> _output_get (Variables|Default|GetPeriodicActivationTime))
        (Variables|Default|SetActive true)
        (goto _label_2)))
    (else
      (bind _output_get_2 (Variables|Default|SetPeriodicTimer (+ (Variables|Default|GetPeriodicTimer) DeltaTime)))
      (if (> _output_get_2 (Variables|Default|GetPeriodicDelay))
        (Variables|Default|SetPeriodicTimer 0.0)
        (Variables|Default|SetPeriodicDelayUsed true)
        (goto _label)))))